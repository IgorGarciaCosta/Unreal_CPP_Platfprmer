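; BP_Falling is an interaction Blueprint with a Paper2D sprite whose opacity can be animated and restored.
; On BeginPlay it creates a dynamic instance of a translucent sprite material and assigns it to the sprite.
; MakeTranslucid plays a timeline that drives the material's Opacity parameter, and ResetOpacity sets it back to fully opaque.
; No falling logic or caller of these events appears in its graphs.
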(event `self.ReceiveBeginPlay`
  (bind _returnvalue (`KismetMaterialLibrary.CreateDynamicMaterialInstance` "/Paper2D/TranslucidBaseSpriteMat_Inst.TranslucidBaseSpriteMat_Inst"))
  (bind _output_get (set `self.MatInstance` _returnvalue))
  (`PrimitiveComponent.SetMaterial` (`self.PaperSprite`) 0 _output_get))

(event `self.MakeTranslucid`
  (bind (_direction _newtrack_0) (`Timeline|Timeline`)
    (:`Update`
      (`MaterialInstanceDynamic.SetScalarParameterValue` (`self.MatInstance`) "Opacity" _newtrack_0))))

(event `self.ResetOpacity`
  (`MaterialInstanceDynamic.SetScalarParameterValue` (`self.MatInstance`) "Opacity" 1.0))

(fn `UserConstructionScript`)